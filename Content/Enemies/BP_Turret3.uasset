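; Enemy turret that shoots at the player and shows a health bar widget.
; Pawn sensing turns it toward a seen third-person character and, after a one-second Delay, spawns a BP_Mermi1 projectile at its arrow.
; Damage lowers clamped health; at zero it plays a sound, drops a puzzle item and sometimes a health pickup, then destroys itself.
; Tick refreshes the bar and rotates it using the camera's rotation.
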(event `self.ReceiveAnyDamage`
  (params (Damage :type "Float (single-precision)") (DamageType :type "DamageType Object Reference") (InstigatedBy :type "Controller Object Reference") (DamageCauser :type "Actor Object Reference"))
  (bind _returnvalue (`self.GetTransform`))
  (`KismetSystemLibrary.PrintString` "Hello")
  (bind _output_get (set `self.Health` (`KismetMathLibrary.FClamp` (- (`self.Health`) Damage) 0.0 (`self.MaxHealth`))))
  (set `/Game/Enemies/WB_Enemies_Health.Health` _output_get (`self.healthbarwidget`))
  (if (== (`self.Health`) 0.0)
    (if (> (`KismetMathLibrary.RandomIntegerInRange` 1 4) 2)
      (`|SpawnActorFromClass` "/Game/Enemies/BP_HealthCollecter.BP_HealthCollecter_C" _returnvalue "Undefined" "MultiplyWithRoot" null null))
    (`GameplayStatics.PlaySound2D` (`self.deathsound`) 1.0 2.0 0.0 null null)
    (`|SpawnActorFromClass` "/Game/Puzzle/BP_PuzzleItem.BP_PuzzleItem_C" _returnvalue "Undefined" "MultiplyWithRoot" null null)
    (`KismetSystemLibrary.Delay` 0.1)
    (`self.K2_DestroyActor`)))

(event `self.ReceiveActorBeginOverlap`
  (params (OtherActor :type "Actor Object Reference")))

(event `self.ReceiveTick`
  (params (DeltaSeconds :type "Float (single-precision)"))
  (bind _healtbarwidget (`self.HealtBarWidget`))
  (bind _aswb_enemies_health (cast `/Game/Enemies/WB_Enemies_Health` (`WidgetComponent.GetUserWidgetObject` (`self.HealtBarWidget`))))
  (bind _output_get (set `self.healthbarwidget` _aswb_enemies_health))
  (set `/Game/Enemies/WB_Enemies_Health.Health` (`self.Health`) _output_get)
  (`SceneComponent.K2_SetWorldRotation` _healtbarwidget (`KismetMathLibrary.FindLookAtRotation` (`SceneComponent.K2_GetComponentLocation` _healtbarwidget) (`KismetMathLibrary.Conv_RotatorToVector` (`SceneComponent.K2_GetComponentRotation` (`PlayerCameraManager.TransformComponent` (`GameplayStatics.GetPlayerCameraManager` 0))))) false false))

(event `self.PawnSensing.OnSeePawn`
  (params (Pawn :type "Pawn Object Reference"))
  (cast `/Game/ThirdPerson/Blueprints/BP_ThirdPersonCharacter` Pawn)
  (`self.K2_SetActorRotation` (`KismetMathLibrary.FindLookAtRotation` (`self.K2_GetActorLocation`) (`self.K2_GetActorLocation` Pawn)))
  (`KismetSystemLibrary.Delay` 1.0)
  (`|SpawnActorFromClass` "/Game/Enemies/BP_Mermi1.BP_Mermi1_C" (`SceneComponent.K2_GetComponentToWorld` (`self.Arrow1`)) "Undefined" "MultiplyWithRoot" null null))

(fn `UserConstructionScript`)