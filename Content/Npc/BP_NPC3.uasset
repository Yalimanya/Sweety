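; BP_NPC3 is an NPC that shows a line-by-line dialogue widget when its Talk event is called.
; Each call advances TalkIndex through the Dialouge array and writes that line into a WB_Dialouge3 widget.
; When UI is invalid it creates the widget, passes it an image and plays a first-see sound; otherwise it plays a switch sound.
; Past the last line it removes the widget and resets the index, without clearing the UI reference.
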(event `self.Talk`
  (`/Engine/EditorBlueprintResources/StandardMacros.IncrementInt` (`self.TalkIndex`)
    (:`  `
      (if (< (`self.TalkIndex`) (`KismetArrayLibrary.Array_Length` (`self.dialouge`)))
        (`self.UI`
          (:`then`
            (`GameplayStatics.PlaySound2D` (`self.SwitchSFX`) 1.0 1.0 0.0 null null))
          (:`else`
            (`GameplayStatics.PlaySound2D` (`self.FirstseeSFX`) 1.0 1.0 0.0 null null)
            (bind _returnvalue (`|CreateWidget` "/Game/Npc/WB_Dialouge3.WB_Dialouge3_C" (`GameplayStatics.GetPlayerController` 0)))
            (bind _output_get (set `self.UI` _returnvalue))
            (`UserWidget.AddToViewport` _output_get 0)
            (set `/Game/Npc/WB_Dialouge3.Return Value Image` (`self.Return Value Image`) (`self.UI`))))
        (`TextBlock.SetText` (`/Game/Npc/WB_Dialouge3.TalkText` (`self.UI`)) (`KismetTextLibrary.Conv_StringToText` (`|GetArrayItem` (`self.dialouge`) (`self.TalkIndex`))))
        (else
          (`Widget.RemoveFromParent` (`self.UI`))
          (set `self.TalkIndex` -1))))))

(fn `UserConstructionScript`)