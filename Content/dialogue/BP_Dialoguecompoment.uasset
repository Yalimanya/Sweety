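; BP_Dialoguecompoment is a dialogue component that runs data-table-driven, branching conversations in a widget.
; Interact creates the dialogue widget with cursor and UI input, advances it on later calls, and removes it once the end flag is set.
; Each row supplies the text, next row and table, and end flag.
; Option buttons spawn only from the opening row and report back through Optionselected, which clears them and jumps to the chosen row.
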(event `CustomEvent`)

(event `Option selected`
  (params (RowName :type Name) (DataTable :type "DataTable Object Reference"))
  (bind _dialougewidget (`self.Dialougewidget`))
  (bind _returnvalue (`|GetDataTableRow` DataTable RowName)
    (:`then`
      (`PanelWidget.ClearChildren` (`/Game/dialogue/WB_Dialouge2.optionscrollbox` _dialougewidget))
      (bind (_dialogue _row _datatable _enddialogue_) (break `/Game/dialogue/Dialouge_Structure` _returnvalue))
      (`/Game/dialogue/WB_Dialouge2.Update Dialogue` _dialougewidget _dialogue)
      (set `self.Row Name` _row)
      (set `self.Data Table` _datatable)
      (set `self.Enddialouge` _enddialogue_))))

(event `/Game/dialogue/BP_Interact.Interact`
  (params (playerref :type "/Game/ThirdPerson/Blueprints/BP_ThirdPersonCharacter Object Reference"))
  (bind _returnvalue (`GameplayStatics.GetPlayerController` 0))
  (bind _returnvalue_2 (`GameplayStatics.GetPlayerController` 0))
  (if (`self.Enddialouge`)
    (`Widget.RemoveFromParent` (`self.Dialougewidget`))
    (set `self.Enddialouge` false)
    (set `self.Dialougewidget` null)
    (`WidgetBlueprintLibrary.SetInputMode_GameOnly` _returnvalue)
    (set `PlayerController.bShowMouseCursor` false _returnvalue)
    (else
      (`/Engine/EditorBlueprintResources/StandardMacros.IsValid` (`self.Dialougewidget`)
        (:`Is Valid`
          (bind _returnvalue_3 (`|GetDataTableRow` (`self.Data Table`) (`self.Row Name`))
            (:`then`
              (bind (_dialogue _row _datatable _enddialogue_) (break `/Game/dialogue/Dialouge_Structure` _returnvalue_3))
              (`/Game/dialogue/WB_Dialouge2.Update Dialogue` (`self.Dialougewidget`) _dialogue)
              (set `self.Row Name` _row)
              (set `self.Data Table` _datatable)
              (set `self.Enddialouge` _enddialogue_))))
        (:`Is Not Valid`
          (bind _returnvalue_4 (`|GetDataTableRow` (`self.Data Table`) (`self.Row Name`))
            (:`then`
              (`KismetSystemLibrary.PrintString` "Hello")
              (bind (_dialogue_2 _row_2 _datatable_2 _enddialogue__2 _openendeddialogue_ _openendendeddialogueoptions) (break `/Game/dialogue/Dialouge_Structure` _returnvalue_4))
              (bind _returnvalue_5 (`|CreateWidget` "/Game/dialogue/WB_Dialouge2.WB_Dialouge2_C" null (`KismetTextLibrary.Conv_NameToText` (`self.Name`)) _dialogue_2))
              (bind _output_get (set `self.Dialougewidget` _returnvalue_5))
              (`UserWidget.AddToViewport` _output_get 0)
              (set `self.Row Name` _row_2)
              (set `self.Data Table` _datatable_2)
              (set `self.Enddialouge` _enddialogue__2)
              (`WidgetBlueprintLibrary.SetInputMode_GameAndUIEx` _returnvalue_2 null)
              (set `PlayerController.bShowMouseCursor` true _returnvalue_2)
              (if _openendeddialogue_
                (for _array_element _openendendeddialogueoptions
                  (bind (_optionname _row_3 _datatable_3) (break `/Game/dialogue/Optionsdialogue_Structure` _array_element))
                  (bind _returnvalue_6 (`|CreateWidget` "/Game/dialogue/WB_Option.WB_Option_C" null (`KismetTextLibrary.Conv_NameToText` _optionname) self _row_3 _datatable_3))
                  (`PanelWidget.AddChild` (`/Game/dialogue/WB_Dialouge2.optionscrollbox` (`self.Dialougewidget`)) _returnvalue_6))))))))))